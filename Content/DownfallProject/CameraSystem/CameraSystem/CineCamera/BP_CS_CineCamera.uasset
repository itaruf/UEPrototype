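; BP_CS_CineCamera is a camera system Blueprint for an ALS player, currently only a partly wired scaffold.
; BeginPlay caches the ALS character, controller and camera manager and calls the third-person pivot target interface.
; Activation events only toggle IsActive; Tick, UpdatePosition and UpdateRotation are empty.
; Logic to follow CustomCameraBehavior or lerp position on a timeline is disconnected and never runs.
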(event `OnActivation`
  (set `self.isActive` true))

(event `OnDeactivation`
  (set `self.isActive` false))

(event `self.ReceiveBeginPlay`
  (bind _asals_anim_man_character_bp (cast `/Game/AdvancedLocomotionV4/Blueprints/CharacterLogic/ALS_AnimMan_CharacterBP` (`GameplayStatics.GetPlayerPawn` 0)))
  (set `self.Player` _asals_anim_man_character_bp)
  (bind _asals_player_controller (cast `/Game/AdvancedLocomotionV4/Blueprints/CharacterLogic/ALS_Player_Controller` (`GameplayStatics.GetPlayerController` 0)))
  (set `self.PlayerController` _asals_player_controller)
  (bind _asals_player_camera_manager (cast `/Game/DownfallProject/CameraSystem/CameraSystem/Blueprints/ALS_PlayerCameraManager` (`PlayerController.PlayerCameraManager` (`self.PlayerController`))))
  (set `self.PlayerCameraManager` _asals_player_camera_manager)
  (message `/Game/AdvancedLocomotionV4/Blueprints/Interfaces/ALS_Camera_BPI.BPI_Get_3P_PivotTarget` (`self.Player`)))

(event `self.ReceiveTick`
  (params (DeltaSeconds :type "Float (single-precision)")))

(event `UpdatePosition`
  (params (Target :type "Vector Structure")))

(event `UpdateRotation`)

(fn `UserConstructionScript`)