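; Base camera trigger in the camera system, which activates its assigned BaseCamera when the Player overlaps it.
; Begin overlap checks that the camera is registered with the PlayerCameraManager and inactive, then deactivates the current camera and activates this one.
; BeginPlay and Tick provide a fallback, activating it after a world-delta delay when no camera is active and the player is inside.
; Leaving the trigger does nothing, as the deactivation logic is unwired.
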(event `self.ReceiveTick`
  (params (DeltaSeconds :type "Float (single-precision)"))
  (`parent.ReceiveTick` DeltaSeconds)
  (`/Engine/EditorBlueprintResources/StandardMacros.IsValid` (`self.Player Camera Manager`) :!label _label
    (:`Is Valid`
      (bind _result (`/Game/DownfallProject/CameraSystem/CameraSystem/Blueprints/ALS_PlayerCameraManager.IsCameraCurrentlyActive` (`self.Player Camera Manager`)))
      (if (not _result)
        (`KismetSystemLibrary.Delay` (`GameplayStatics.GetWorldDeltaSeconds`))
        (`/Engine/EditorBlueprintResources/StandardMacros.IsValid` (`self.Player`)
          (:`Is Valid`
            (`/Engine/EditorBlueprintResources/StandardMacros.IsValid` (`self.BaseCamera`)
              (:`Is Valid`
                (if (and (`self.IsOverlappingActor` (`self.Player`)) (not (`/Game/DownfallProject/CameraSystem/CameraSystem/BaseCamera/Parent/BP_CS_BaseCamera.isActive` (`self.BaseCamera`))))
                  (`/Game/DownfallProject/CameraSystem/CameraSystem/BaseCamera/Parent/BP_CS_BaseCamera.On Activation` (`self.BaseCamera`)))))))))))

(event `self.ReceiveBeginPlay`
  (`parent.ReceiveBeginPlay`)
  (goto _label))

(event `self.ReceiveActorBeginOverlap`
  (params (OtherActor :type "Actor Object Reference"))
  (`/Engine/EditorBlueprintResources/StandardMacros.IsValid` (`self.Player`)
    (:`Is Valid`
      (if (== OtherActor (`self.Player`))
        (`/Engine/EditorBlueprintResources/StandardMacros.IsValid` (`self.Player Camera Manager`)
          (:`Is Valid`
            (`/Engine/EditorBlueprintResources/StandardMacros.IsValid` (`self.BaseCamera`)
              (:`Is Valid`
                (if (!= (`KismetArrayLibrary.Array_Find` (`/Game/DownfallProject/CameraSystem/CameraSystem/Blueprints/ALS_PlayerCameraManager.Cameras` (`self.Player Camera Manager`)) (`self.BaseCamera`)) -1)
                  (if (not (`/Game/DownfallProject/CameraSystem/CameraSystem/BaseCamera/Parent/BP_CS_BaseCamera.isActive` (`self.BaseCamera`)))
                    (`/Game/DownfallProject/CameraSystem/CameraSystem/Blueprints/ALS_PlayerCameraManager.Deactivate Current Camera` (`self.Player Camera Manager`))
                    (`/Game/DownfallProject/CameraSystem/CameraSystem/BaseCamera/Parent/BP_CS_BaseCamera.On Activation` (`self.BaseCamera`))))))))))))

(event `self.ReceiveActorEndOverlap`
  (params (OtherActor :type "Actor Object Reference")))

(fn `UserConstructionScript`
  (`parent.UserConstructionScript`))