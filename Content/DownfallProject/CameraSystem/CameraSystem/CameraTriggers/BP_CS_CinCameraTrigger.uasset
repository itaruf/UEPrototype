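; BP_CS_CinCameraTrigger is a camera system trigger meant to tie a cinematic camera to a Level Sequence.
; On BeginPlay it creates a sequence player from LevelSequenceReference, if valid, and stores the LevelSequenceActor.
; Logic to play or stop the sequence and activate or deactivate CineCamera for the Player is disconnected and never runs.
; Both overlap events are empty, so this graph never starts playback.
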(event `self.ReceiveBeginPlay`
  (`/Engine/EditorBlueprintResources/StandardMacros.IsValid` (`self.LevelSequenceReference`)
    (:`Is Valid`
      (bind _outactor (`LevelSequencePlayer.CreateLevelSequencePlayer` (`self.LevelSequenceReference`)))
      (set `self.LevelSequenceActor` _outactor))))

(event `self.ReceiveActorBeginOverlap`
  (params (OtherActor :type "Actor Object Reference")))

(event `self.ReceiveActorEndOverlap`
  (params (OtherActor :type "Actor Object Reference")))

(fn `UserConstructionScript`
  (`parent.UserConstructionScript`))