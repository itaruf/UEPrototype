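; Free-follow camera in the camera system, built on a parent camera class and switched on through an Activation interface event.
; Activation applies the preset, starts a looping frame-interval timer, turns off the camera manager's autopilot and passes it the relative camera target.
; It then either cuts to position or updates FOV and interpolates there.
; The essential-values and current-state interface getters return only defaults.
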(event `/Game/DownfallProject/CameraSystem/Interfaces/BPI_Activation.Activation`
  ;[0.4336 0.349 1] Interface Event : Activation
  (`self.Event Set Values On Activation`)
  (if (`self.Cut`)
    (`|ExecutionSequence`
      (:`then_0`
        (`self.Event Update Position (Cut)`))
      (:`then_1`
        (`/Engine/EditorBlueprintResources/StandardMacros.IsValid` (`self.PlayerCameraManager`)
          (:`Is Valid`
            (`/Engine/EditorBlueprintResources/StandardMacros.IsValid` (`self.CameraComponent`))))))
    (else
      ;;[1 1 1] Update FOV During Camera Transion
      (`self.Update FOV`)
      (`self.Event Update Position (Interpolation)`))))

(event `Event Set Values On Activation`
  ;[0.3992 1 0.9901] Event Set Values On Activation
  (`|ExecutionSequence`
    (:`then_0`
      (set `self.isActive` true)
      (`self.SetPreset`)
      (`KismetSystemLibrary.PrintString` (`KismetStringLibrary.Concat_StrStr` (`KismetSystemLibrary.GetDisplayName` self) " activated"))
      (bind _returnvalue (`KismetSystemLibrary.K2_SetTimerDelegate` (`|CreateDelegate` :!event `Event Update Preset`) (`GameplayStatics.GetWorldDeltaSeconds`) true))
      (set `self.SetPresetTimer` _returnvalue))
    (:`then_1`
      (`/Engine/EditorBlueprintResources/StandardMacros.IsValid` (`self.PlayerCameraManager`)
        (:`Is Valid`
          (set `/Game/DownfallProject/CameraSystem/Blueprints/ALS_PlayerCameraManager.isAutoPiloteActivated` false (`self.PlayerCameraManager`)))))
    (:`then_2`
      (`/Engine/EditorBlueprintResources/StandardMacros.IsValid` (`self.PlayerCameraManager`)
        (:`Is Valid`
          (set `/Game/DownfallProject/CameraSystem/Blueprints/ALS_PlayerCameraManager.Camera Target (Relative)` (`self.Camera Target (Relative)`) (`self.PlayerCameraManager`)))))))

(fn `BPI_Get_CurrentStates`
  (returns (PawnMovementMode :type "EMovementMode Enum") (MovementState :type "/Game/AdvancedLocomotionV4/Data/Enums/ALS_MovementState Enum") (PrevMovementState :type "/Game/AdvancedLocomotionV4/Data/Enums/ALS_MovementState Enum") (MovementAction :type "/Game/AdvancedLocomotionV4/Data/Enums/ALS_MovementAction Enum") (RotationMode :type "/Game/AdvancedLocomotionV4/Data/Enums/ALS_RotationMode Enum") (ActualGait :type "/Game/AdvancedLocomotionV4/Data/Enums/ALS_Gait Enum") (ActualStance :type "/Game/AdvancedLocomotionV4/Data/Enums/ALS_Stance Enum") (ViewMode :type "/Game/AdvancedLocomotionV4/Data/Enums/ALS_ViewMode Enum") (OverlayState :type "/Game/AdvancedLocomotionV4/Data/Enums/ALS_OverlayState Enum") (WallRunSide :type "/Game/AdvancedLocomotionV4/Data/Enums/WallRunSide Enum"))
  (return "MOVE_None" "NewEnumerator0" "NewEnumerator0" "NewEnumerator4" "NewEnumerator0" "NewEnumerator0" "NewEnumerator0" "NewEnumerator0" "NewEnumerator0" "NewEnumerator0"))

(fn `BPI_Get_EssentialValues`
  (returns (Velocity :type "Vector Structure") (Acceleration :type "Vector Structure") (MovementInput :type "Vector Structure") (IsMoving :type Boolean) (HasMovementInput :type Boolean) (Speed :type "Float (double-precision)") (MovementInputAmount :type "Float (double-precision)") (AimingRotation :type "Rotator Structure") (AimYawRate :type "Float (double-precision)"))
  (return (0.0 0.0 0.0) (0.0 0.0 0.0) (0.0 0.0 0.0) false false 0.0 0.0 (struct) 0.0))

(fn `UserConstructionScript`
  (`parent.UserConstructionScript`))