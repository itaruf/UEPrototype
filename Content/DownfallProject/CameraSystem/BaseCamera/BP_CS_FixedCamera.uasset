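; Fixed camera actor that, while active, supplies target rotation, field of view and location to the player camera manager.
; Each tick restarts a look-at timeline toward the player, though its lerp alpha is multiplied by zero, leaving rotation unchanged.
; The location target either snaps to the actor when Cut is set or lerps there through a timeline restarted every tick.
; Activation and deactivation only print debug messages.
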(event `self.ReceiveTick`
  (params (DeltaSeconds :type "Float (single-precision)"))
  (`parent.ReceiveTick` DeltaSeconds)
  (`self.UpdateRotation` (`self.Player`))
  (if (`self.isActive`)
    (set `/Game/DownfallProject/CameraSystem/Blueprints/ALS_PlayerCameraManager.TargetCameraRotation` (`self.K2_GetActorRotation`) (`self.PlayerCameraManager`))
    (set `/Game/DownfallProject/CameraSystem/Blueprints/ALS_PlayerCameraManager.TargetCameraFOV` (`CameraComponent.FieldOfView` (`self.CameraComponent`)) (`self.PlayerCameraManager`))
    (if (`self.Cut`)
      (set `/Game/DownfallProject/CameraSystem/Blueprints/ALS_PlayerCameraManager.TargetCameraLocation` (`self.K2_GetActorLocation`) (`self.PlayerCameraManager`))
      (else
        (`self.UpdatePosition` (`self.Player`))))))

(event `UpdateRotation`
  (params (Target :type "Actor Object Reference"))
  (bind (_direction _value) (`Timeline|0 to 1 (2)` :!via `PlayFromStart`)
    (:`Update`
      (`self.K2_SetActorRotation` (`KismetMathLibrary.RLerp` (`self.K2_GetActorRotation`) (`KismetMathLibrary.FindLookAtRotation` (`self.K2_GetActorLocation`) (`self.K2_GetActorLocation` Target)) (* _value 0.0))))))

(event `UpdatePosition`
  (params (Target :type "Actor Object Reference"))
  (bind (_direction _value) (`Timeline|0 to 1` :!via `PlayFromStart`)
    (:`Update`
      (set `/Game/DownfallProject/CameraSystem/Blueprints/ALS_PlayerCameraManager.TargetCameraLocation` (`KismetMathLibrary.VLerp` (`/Game/DownfallProject/CameraSystem/Blueprints/ALS_PlayerCameraManager.TargetCameraLocation` (`self.PlayerCameraManager`)) (`self.K2_GetActorLocation`) _value) (`self.PlayerCameraManager`)))))

(event `/Game/DownfallProject/CameraSystem/Interfaces/BPI_Activation.Activation`
  (`KismetSystemLibrary.PrintString` (`KismetStringLibrary.Concat_StrStr` (`KismetSystemLibrary.GetDisplayName` self) " activated")))

(event `/Game/DownfallProject/CameraSystem/Interfaces/BPI_Deactivation.Deactivation`
  (`KismetSystemLibrary.PrintString` (`KismetStringLibrary.Concat_StrStr` (`KismetSystemLibrary.GetDisplayName` self) " deactivated")))

(fn `UserConstructionScript`
  (`parent.UserConstructionScript`))