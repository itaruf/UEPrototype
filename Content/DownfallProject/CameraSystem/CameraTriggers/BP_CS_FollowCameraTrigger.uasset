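; Camera trigger that switches the view to a free-follow camera for the player.
; Spawning creates a BP_CS_FreeFollowCamera attached to the trigger and registers it with the PlayerCameraManager.
; Player overlap swaps from the current camera to this registered one if it is inactive.
; Activation spawns the camera if missing and, after a frame-length delay, takes over when no camera is active and the player is already inside.
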(event `Event Spawn Camera`
  (bind (_returnvalue_location _returnvalue_rotation) (`KismetMathLibrary.BreakTransform` (`self.GetTransform`)))
  ;[1 0.5284 0.8962] Event Spawn Camera
  (bind _returnvalue (`|SpawnActorFromClass` "/Game/DownfallProject/CameraSystem/BaseCamera/BP_CS_FreeFollowCamera.BP_CS_FreeFollowCamera_C" (`KismetMathLibrary.MakeTransform` _returnvalue_location _returnvalue_rotation) "Undefined" "OverrideRootScale" null null))
  (bind _output_get (set `self.BaseCamera` _returnvalue))
  (`self.K2_AttachToActor` _output_get self "None" "SnapToTarget" "SnapToTarget" "KeepRelative" true)
  (`KismetArrayLibrary.Array_Add` (`/Game/DownfallProject/CameraSystem/Blueprints/ALS_PlayerCameraManager.Cameras` (`self.Player Camera Manager`)) _output_get)
  (`/Game/DownfallProject/CameraSystem/BaseCamera/Parent/BP_CS_BaseCamera.Event Set Data` _output_get))

(event `self.ReceiveBeginPlay`
  ;[1 0.5639 0.4129] Event Begin Play
  (`parent.ReceiveBeginPlay`))

(event `self.ReceiveActorBeginOverlap`
  (params (OtherActor :type "Actor Object Reference"))
  ;[0.631 1 0.6133] Event Begin Overlap
  (`/Engine/EditorBlueprintResources/StandardMacros.IsValid` OtherActor
    (:`Is Valid`
      (if (== OtherActor (`self.Player`))
        (`/Engine/EditorBlueprintResources/StandardMacros.IsValid` (`self.Player`)
          (:`Is Valid`
            (`/Engine/EditorBlueprintResources/StandardMacros.IsValid` (`self.Player Camera Manager`)
              (:`Is Valid`
                (bind _result (`/Game/DownfallProject/CameraSystem/Blueprints/ALS_PlayerCameraManager.IsCameraCurrentlyActive` (`self.Player Camera Manager`)))
                (if _result
                  (`/Engine/EditorBlueprintResources/StandardMacros.IsValid` (`self.BaseCamera`)
                    (:`Is Valid`
                      (if (!= (`KismetArrayLibrary.Array_Find` (`/Game/DownfallProject/CameraSystem/Blueprints/ALS_PlayerCameraManager.Cameras` (`self.Player Camera Manager`)) (`self.BaseCamera`)) -1)
                        (if (not (`/Game/DownfallProject/CameraSystem/BaseCamera/Parent/BP_CS_BaseCamera.isActive` (`self.BaseCamera`)))
                          (`/Game/DownfallProject/CameraSystem/Blueprints/ALS_PlayerCameraManager.Deactivate Current Camera` (`self.Player Camera Manager`))
                          (`/Game/DownfallProject/CameraSystem/BaseCamera/Parent/BP_CS_BaseCamera.On Activation` (`self.BaseCamera`))
                          (`/Game/DownfallProject/CameraSystem/Blueprints/ALS_PlayerCameraManager.Event Set Current Camera` (`self.Player Camera Manager`) (`self.BaseCamera`)))))))))))))))

(event `self.ReceiveTick`
  (params (DeltaSeconds :type "Float (single-precision)"))
  ;[0.631 1 0.6133] Event Begin Overlap
  ;;[1 1 1] Actor already is within the trigger range
)

(event `/Game/DownfallProject/CameraSystem/Interfaces/BPI_Activation.Activation`
  ;[0.631 1 0.6133] Event Begin Overlap
  ;;[1 1 1] Actor already is within the trigger range
  (`/Engine/EditorBlueprintResources/StandardMacros.IsValid` (`self.BaseCamera`)
    (:`Is Valid`
      _)
    (:`Is Not Valid`
      (`self.Event Spawn Camera`)))
  (`/Engine/EditorBlueprintResources/StandardMacros.IsValid` (`self.Player Camera Manager`)
    (:`Is Valid`
      (`KismetSystemLibrary.Delay` (`GameplayStatics.GetWorldDeltaSeconds`))
      (bind _result (`/Game/DownfallProject/CameraSystem/Blueprints/ALS_PlayerCameraManager.IsCameraCurrentlyActive` (`self.Player Camera Manager`)))
      (if (not _result)
        (`/Engine/EditorBlueprintResources/StandardMacros.IsValid` (`self.Player`)
          (:`Is Valid`
            (if (and (`self.IsOverlappingActor` (`self.Player`)) (not (`/Game/DownfallProject/CameraSystem/BaseCamera/Parent/BP_CS_BaseCamera.isActive` (`self.BaseCamera`))))
              (`/Game/DownfallProject/CameraSystem/Blueprints/ALS_PlayerCameraManager.Deactivate Current Camera` (`self.Player Camera Manager`))
              (`/Game/DownfallProject/CameraSystem/BaseCamera/Parent/BP_CS_BaseCamera.On Activation` (`self.BaseCamera`))
              (`/Game/DownfallProject/CameraSystem/Blueprints/ALS_PlayerCameraManager.Event Set Current Camera` (`self.Player Camera Manager`) (`self.BaseCamera`)))))))))

(fn `UserConstructionScript`
  (`parent.UserConstructionScript`))