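; Fire prop Blueprint that turns to face the player's camera and flickers its point light.
; On BeginPlay, a Light timeline drives the point light intensity from its Flicker track scaled by LightIntensity.
; A looping timer calls GetAngle every tenth of a second, billboarding the whole actor along the normalized, slightly offset vector toward the camera, rather than updating on Tick.
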(event `self.ReceiveBeginPlay`
  (`KismetSystemLibrary.K2_SetTimer` null "GetAngle" 0.1 true)
  (bind (_direction _flicker) (`Timeline|Light`)
    (:`Update`
      (`LightComponent.SetIntensity` (`self.PointLight`) (* _flicker (`self.Light Intensity`))))))

(fn `GetAngle`
  (`self.K2_SetActorRotation` (`KismetMathLibrary.Conv_VectorToRotator` (`KismetMathLibrary.Normal` (- (- (`PlayerCameraManager.GetCameraLocation` (`GameplayStatics.GetPlayerCameraManager` 0)) (`self.K2_GetActorLocation`)) (1.0 1.0 0.0))))))

(fn `UserConstructionScript`)