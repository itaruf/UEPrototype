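; InputReader is an actor that captures player input into variables.
; On BeginPlay it enables input from player controller 0.
; WallRun and JumpAction press and release events set the L2Pressed and R2Pressed flags.
; Each tick it copies the ControlTailUpDown and ControlTailLeftRight axis values into TailUpDown and TailLeftRight.
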(event `self.ReceiveBeginPlay`
  (`self.EnableInput` (`GameplayStatics.GetPlayerController` 0)))

(event `InputAction|WallRun`
  (params (Key :type "Key Structure"))
  (:`Pressed`
    (set `self.L2Pressed` true))
  (:`Released`
    (set `self.L2Pressed` false)))

(event `InputAction|JumpAction`
  (params (Key :type "Key Structure"))
  (:`Pressed`
    (set `self.R2Pressed` true))
  (:`Released`
    (set `self.R2Pressed` false)))

(event `self.ReceiveTick`
  (params (DeltaSeconds :type "Float (single-precision)"))
  (set `self.TailUpDown` (`self.GetInputAxisValue`))
  (set `self.TailLeftRight` (`self.GetInputAxisValue`)))

(fn `UserConstructionScript`)